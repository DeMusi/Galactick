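; Enemy spawner that creates two enemy types and asteroids at random X/Z points in its collision bounds, locked to its own Y.
; When enabled, looping one-second timers drive the spawn events.
; Basic enemies spawn after random delays under the BP_GameMode enemy cap, also triggering the second type at each new even kill count.
; Asteroid spawning loops a random count through random delays, ignoring the cap.
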(event `self.ReceiveBeginPlay`
  (bind _asbp_game_mode (cast `/Game/Blueprint/BP_GameMode` (`GameplayStatics.GetGameMode`)))
  (set `self.BP_Gamemode` _asbp_game_mode)
  (if (`self.SpawnEnemies`)
    (`|ExecutionSequence`
      (:`then_0`
        (`KismetSystemLibrary.K2_SetTimer` null "SpawnEnemy" 1.0 true))
      (:`then_1`
        (`KismetSystemLibrary.K2_SetTimer` null "SpawnActeroid" 1.0 true))
      (:`then_2`
        (`KismetSystemLibrary.K2_SetTimer` null "SpawnEnemy 2" 1.0 true)))))

(event `SpawnEnemy`
  (bind _bp_gamemode (`self.BP_GameMode`))
  (bind _enemieskilled (`/Game/Blueprint/BP_GameMode.EnemiesKilled` _bp_gamemode))
  ;[1 1 1] SpawnEmey1
  (if (< (`/Game/Blueprint/BP_GameMode.EnemyCount` _bp_gamemode) (`/Game/Blueprint/BP_GameMode.MaxEnemies` _bp_gamemode))
    (if (and (== (mod _enemieskilled 2) 0) (!= _enemieskilled (`self.CurrentEnemiesKilled`)))
      (`self.Spawn Enemy 2`))
    (`KismetSystemLibrary.Delay` (`KismetMathLibrary.RandomFloatInRange` 0.5 2.0))
    (`|SpawnActorFromClass` "/Game/Blueprint/Enemies/BP_EnemyBase_One.BP_EnemyBase_One_C" (`KismetMathLibrary.MakeTransform` (`self.Get random loc`)) "Undefined" "OverrideRootScale" null null)))

(event `Spawn Enemy 2`
  ;[1 1 1] Spawn enemy2
  (set `self.CurrentEnemiesKilled` (`/Game/Blueprint/BP_GameMode.EnemiesKilled` (`self.BP_GameMode`)))
  (`|SpawnActorFromClass` "/Game/Blueprint/Enemies/BP_EnemyBase_Two.BP_EnemyBase_Two_C" (`KismetMathLibrary.MakeTransform` (`self.Get random loc`)) "Undefined" "OverrideRootScale" null null))

(event `SpawnActeroid`
  (for _ (range (+ (`KismetMathLibrary.RandomIntegerInRange` 1 3) 1))
    (`KismetSystemLibrary.Delay` (`KismetMathLibrary.RandomFloatInRange` 0.5 3.0))
    (`|SpawnActorFromClass` "/Game/Blueprint/Enemies/BP_EnemyBase_Acteroid.BP_EnemyBase_Acteroid_C" (`KismetMathLibrary.MakeTransform` (`self.Get random loc`)) "Undefined" "OverrideRootScale" null null)))

(fn `Get random loc`
  (returns (Location :type "Vector Structure"))
  (bind (_returnvalue_x _returnvalue_y) (`KismetMathLibrary.BreakVector` (`self.K2_GetActorLocation`)))
  (bind (_origin _boxextent) (`KismetSystemLibrary.GetComponentBounds` (`self.CollisionComponent`)))
  (bind (_returnvalue_x_2 _returnvalue_y_2 _returnvalue_z) (`KismetMathLibrary.BreakVector` (`KismetMathLibrary.RandomPointInBoundingBox` _origin _boxextent)))
  (return (`KismetMathLibrary.MakeVector` _returnvalue_x_2 _returnvalue_y _returnvalue_z)))

(fn `UserConstructionScript`)