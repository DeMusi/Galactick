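; BP_EnemyBase_Two is an enemy Blueprint that delays collision on its StaticMesh after spawning.
; The Construction Script runs the parent's version, applies the Scale variable as the mesh's world scale and disables its collision.
; BeginPlay calls the parent, waits one second, then enables query and physics collision on the mesh.
; The overlap and Tick events are disabled stubs.
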(event `self.ReceiveBeginPlay`
  (`parent.ReceiveBeginPlay`)
  (`KismetSystemLibrary.Delay` 1.0)
  (`PrimitiveComponent.SetCollisionEnabled` (`self.StaticMesh`) "QueryAndPhysics"))

(fn `UserConstructionScript`
  (`parent.UserConstructionScript`)
  (`SceneComponent.SetWorldScale3D` (`self.StaticMesh`) (`self.Scale`))
  (`PrimitiveComponent.SetCollisionEnabled` (`self.StaticMesh`) "NoCollision"))