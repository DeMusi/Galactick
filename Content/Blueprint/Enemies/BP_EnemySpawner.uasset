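; BP_EnemySpawner is an actor that keeps spawning enemies while the game mode's enemy count is below its maximum.
; On BeginPlay it caches BP_GameMode and starts a looping timer that spawns a BP_EnemyBase_One after a short random delay.
; When the kill count reaches a new multiple of five, it also spawns a BP_EnemyBase_Two, recording that count to avoid repeats.
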(event `self.ReceiveBeginPlay`
  (bind _asbp_game_mode (cast `/Game/Blueprint/BP_GameMode` (`GameplayStatics.GetGameMode`)))
  (set `self.BP_GameMode` _asbp_game_mode)
  (`|ExecutionSequence`
    (:`then_0`
      (`KismetSystemLibrary.K2_SetTimer` null "SpawnEnemy" 1.0 true))))

(event `SpawnEnemy`
  (bind _bp_gamemode (`self.BP_GameMode`))
  (bind _enemieskilled (`/Game/Blueprint/BP_GameMode.EnemiesKilled` _bp_gamemode))
  (if (< (`/Game/Blueprint/BP_GameMode.EnemyCount` _bp_gamemode) (`/Game/Blueprint/BP_GameMode.MaxEnemies` _bp_gamemode))
    (if (and (== (mod _enemieskilled 5) 0) (!= _enemieskilled (`self.CurrentEnemiesKilled`)))
      (`self.SpawnEnemy2`))
    (`KismetSystemLibrary.Delay` (`KismetMathLibrary.RandomFloatInRange` 0.5 2.0))
    (`|SpawnActorFromClass` "/Game/Blueprint/Enemies/BP_EnemyBase_One.BP_EnemyBase_One_C" (`KismetMathLibrary.MakeTransform` (0.0 0.0 0.0)) "Undefined" "OverrideRootScale" null null)))

(event `SpawnEnemy2`
  (set `self.CurrentEnemiesKilled` (`/Game/Blueprint/BP_GameMode.EnemiesKilled` (`self.BP_GameMode`)))
  (`|SpawnActorFromClass` "/Game/Blueprint/Enemies/BP_EnemyBase_Two.BP_EnemyBase_Two_C" (`KismetMathLibrary.MakeTransform` (0.0 0.0 0.0)) "Undefined" "OverrideRootScale" null null))

(fn `UserConstructionScript`)