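; Player pawn for an X/Z-plane shooter, with a timeline spin-and-rise spawn that unlocks firing when finished.
; Axis input or, under NewControl, the last touch point drives interpolated speeds that Tick applies with sweeps, yawing the mesh and bouncing off hits.
; Looping timers repeat single-muzzle primary fire (also HUD-triggered) and twin-muzzle secondary fire.
; Damage shakes the camera via BP_GameMode; zero health explodes the pawn and calls GameOver.
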(event `InputAxis|MoveUp`
  (params (AxisValue :type "Float (single-precision)"))
  ;[1 1 1] PlayerInput
  (if (not (`self.new control`))
    (bind _returnvalue (`self.Movemet` AxisValue (`self.VertSpeed`)))
    (set `self.VertSpeed` _returnvalue)))

(event `self.ReceiveBeginPlay`
  (bind _spawnlocation (`self.SpawnLocation`))
  ;[1 1 1] Player Spawn Animation
  (bind _asbp_game_mode (cast `/Game/Blueprint/BP_GameMode` (`GameplayStatics.GetGameMode`)))
  (set `self.BP_GameMode` _asbp_game_mode)
  (set `self.Yaw` (.yaw (`self.K2_GetActorRotation`)))
  (set `self.SpawnLocation` (`self.K2_GetActorLocation`))
  (bind (_direction _speed) (`Timeline|SpawnActorLocation`)
    (:`Update`
      (`self.K2_SetActorLocation` (`KismetMathLibrary.VLerp` _spawnlocation (+ _spawnlocation (0.0 0.0 60.0)) _speed))
      (`SceneComponent.K2_SetRelativeRotation` (`self.PlayerMesh`) (`KismetMathLibrary.RLerp` (struct) (`KismetMathLibrary.MakeRotator` 0.0 0.0 (+ (`self.Yaw`) (`self.SpawnSpinCount`))) _speed) false false))
    (:`Finished`
      (set `self.MoveEnable` true))))

(event `InputAxis|MoveRight`
  (params (AxisValue :type "Float (single-precision)"))
  ;[1 1 1] PlayerInput
  (if (not (`self.new control`))
    (bind _returnvalue (`self.Movemet` AxisValue (`self.HozSpeed`)))
    (set `self.HozSpeed` _returnvalue)))

(event `self.ReceiveTick`
  (params (DeltaSeconds :type "Float (single-precision)"))
  (bind _playermesh (`self.PlayerMesh`))
  (bind _x (.x (`self.K2_GetActorLocation`)))
  (bind _z (.z (`self.K2_GetActorLocation`)))
  (bind _returnvalue (`KismetMathLibrary.Round` _x))
  (bind _returnvalue_2 (`KismetMathLibrary.Round` _z))
  ;[1 1 1] Movement
  (`|ExecutionSequence`
    (:`then_0`
      (set `self.DeltaSeconds` DeltaSeconds)
      (`self.K2_SetActorLocation` (+ (`self.K2_GetActorLocation`) (`KismetMathLibrary.MakeVector` (`self.HozSpeed`))) true)
      (`self.K2_SetActorLocation` (+ (`self.K2_GetActorLocation`) (`KismetMathLibrary.MakeVector` 0.0 0.0 (`self.VertSpeed`))) true)
      (`/Engine/EditorBlueprintResources/StandardMacros.IsValid` self
        (:`Is Valid`
          (`SceneComponent.K2_SetRelativeRotation` _playermesh (`KismetMathLibrary.RInterpTo_Constant` (`SceneComponent.RelativeRotation` _playermesh) (`KismetMathLibrary.MakeRotator` 0.0 0.0 (+ (* (`self.HozSpeed`) -7.0) (`self.Yaw`))) (`self.DeltaSeconds`) 80.0) false false))))
    (:`then_1`
      ;[1 1 1] New control
      (if (`self.new control`)
        (`|ExecutionSequence`
          (:`then_0`
            (if (not (and (`KismetMathLibrary.InRange_IntInt` (- (`self.last touched x`) _returnvalue) -10) (`KismetMathLibrary.InRange_IntInt` (- (`self.last touched y(or z)`) _returnvalue_2) -5 5)))
              (bind _returnvalue_3 (`self.Movemet` (select `bool` (> (- (`self.last touched x`) _returnvalue) 0) :`false` -1.0 :`true` 1.0 :!type "Float (single-precision)") (`self.HozSpeed`)))
              (set `self.HozSpeed` _returnvalue_3)
              (bind _returnvalue_4 (`self.Movemet` (select `bool` (> (- (`self.last touched y(or z)`) _returnvalue_2) 0) :`false` -1.0 :`true` 1.0 :!type "Float (single-precision)") (`self.VertSpeed`)))
              (set `self.VertSpeed` _returnvalue_4)))
          (:`then_1`
            (if (`self.show debub coord`)
              (`TextRenderComponent.K2_SetText` (`self.debug coord`) (`KismetTextLibrary.Conv_StringToText` (`KismetStringLibrary.Concat_StrStr` "X: " (`KismetStringLibrary.Conv_IntToString` (`KismetMathLibrary.Round` _x)) " Z: " (`KismetStringLibrary.Conv_IntToString` (`KismetMathLibrary.Round` _z))))))))))))

(event `PrimFire`
  ;[1 1 1] Primary Fire
  (`self.PrimaryFire` (`SceneComponent.K2_GetComponentToWorld` (`self.ProjectileSpwan`)) :!label _label))

(event `InputAction|PrimaryFire`
  (params (Key :type "Key Structure"))
  ;[1 1 1] Primary Fire
  (:`Pressed`
    (if (`self.MoveEnable`) :!label _label_2
      (`KismetSystemLibrary.K2_SetTimer` null "PrimFire" 0.07 true)
      (goto _label)))
  (:`Released`
    (`KismetSystemLibrary.K2_ClearTimer` null "PrimFire" :!label _label_3)))

(event `Hud fire input`
  (params (isPressed :type Boolean))
  ;[1 1 1] Primary Fire
  (if isPressed
    (goto _label_2)
    (else
      (goto _label_3))))

(event `SecFire`
  (`self.SecondaryFire` (`SceneComponent.K2_GetComponentToWorld` (`self.ProjectileSpwanL`)) :!label _label_4)
  (`self.SecondaryFire` (`SceneComponent.K2_GetComponentToWorld` (`self.ProjectileSpawnR`))))

(event `InputAction|SecondaryFire`
  (params (Key :type "Key Structure"))
  (:`Pressed`
    (if (`self.MoveEnable`)
      (`KismetSystemLibrary.K2_SetTimer` null "SecFire" 0.2 true)
      (goto _label_4)))
  (:`Released`
    (`KismetSystemLibrary.K2_ClearTimer` null "SecFire")))

(event `InputTouch`
  (params (Location :type "Vector Structure") (FingerIndex :type "ETouchIndex Enum"))
  ;[1 1 1] New control
  (:`Pressed`
    (if (`self.new control`) :!label _label_5
      (bind _returnvalue (`GameUserSettings.GetGameUserSettings`))
      (bind (_x _y) (break `IntPoint` (`GameUserSettings.GetScreenResolution` _returnvalue)))
      (set `self.last touched x` (- (`KismetMathLibrary.Round` (.x Location)) (/ _x 2)))
      (set `self.last touched y(or z)` (`KismetMathLibrary.Round` (* (- (`KismetMathLibrary.Round` (.y Location)) (/ _y 2)) -0.5)))
      (if (`self.show debub coord`)
        (`KismetSystemLibrary.PrintString` (`KismetStringLibrary.Concat_StrStr` "X: " (`KismetStringLibrary.Conv_IntToString` (`self.last touched x`))))
        (`KismetSystemLibrary.PrintString` (`KismetStringLibrary.Concat_StrStr` "Z: " (`KismetStringLibrary.Conv_IntToString` (`self.last touched y(or z)`)))))))
  (:`Released`
    (goto _label_5))
  (:`Moved`
    (goto _label_5)))

(event `self.ReceiveAnyDamage`
  (params (Damage :type "Float (single-precision)") (DamageType :type "DamageType Object Reference") (InstigatedBy :type "Controller Object Reference") (DamageCauser :type "Actor Object Reference"))
  (bind _returnvalue (`self.K2_GetActorLocation`))
  (bind _bp_gamemode (`self.BP_GameMode`))
  (set `self.Health` (`KismetMathLibrary.FClamp` (- (`self.Health`) Damage) 0.0 (`self.MaxHealth`)))
  (`/Game/Blueprint/BP_GameMode.PlayCamSnake` (`self.BP_GameMode`) "/Game/Blueprint/BP_CamSnakeSmall.BP_CamSnakeSmall_C" (`self.K2_GetActorLocation`))
  (if (<= (`self.Health`) 0.0)
    (`GameplayStatics.SpawnEmitterAtLocation` "/Game/Asset/Particles/P_Pixel_Explosion.P_Pixel_Explosion" _returnvalue (struct) (1.0 1.0 1.0) false)
    (`GameplayStatics.PlaySoundAtLocation` "/Game/Asset/Audio/Explodion/ExplosionCue.ExplosionCue" _returnvalue (struct) 1.0 1.0 0.0 null null null)
    (`/Game/Blueprint/BP_GameMode.PlayCamSnake` _bp_gamemode "/Game/Blueprint/BP_CamSnake.BP_CamSnake_C" (`self.K2_GetActorLocation`))
    (`/Game/Blueprint/BP_GameMode.GameOver` _bp_gamemode)
    (`self.K2_DestroyActor`)))

(event `self.Box.OnComponentHit`
  (params (HitComponent :type "PrimitiveComponent Object Reference") (OtherActor :type "Actor Object Reference") (OtherComp :type "PrimitiveComponent Object Reference") (NormalImpulse :type "Vector Structure") (Hit :type "HitResult Structure (by ref)"))
  (set `self.HozSpeed` (* (* (`KismetMathLibrary.Abs` (`self.HozSpeed`)) 2.0) (.x Hit_Normal)))
  (set `self.VertSpeed` (* (* (`KismetMathLibrary.Abs` (`self.VertSpeed`)) 2.0) (.z Hit_Normal))))

(fn `Movemet`
  (params (Direction :type "Float (double-precision)") (Speed :type "Float (double-precision)"))
  (returns (ReturnValue :type "Float (double-precision)"))
  (return (`KismetMathLibrary.FInterpTo` Speed (* (* Direction (`self.MovementSpeed`)) (`self.DeltaSeconds`)) (`self.DeltaSeconds`) 6.0)))

(fn `PrimaryFire`
  (params (SpawnTransform :type "Transform Structure"))
  (locals (ProjectColor :type "LinearColor Structure" :default (struct :`G` 0.025064 :`B` 0.822917)))
  (`|SpawnActorFromClass` "/Game/Blueprint/BP_Project_Primary.BP_Project_Primary_C" SpawnTransform "AlwaysSpawn" "OverrideRootScale" null (`local.ProjectColor`) self)
  (`GameplayStatics.PlaySoundAtLocation` "/Game/Asset/Audio/PlayerShot/Laser_Shoot7.Laser_Shoot7" (`self.K2_GetActorLocation`) (struct) 1.0 1.0 0.0 null null null))

(fn `SecondaryFire`
  (params (Spawn :type "Transform Structure"))
  (locals (Colour :type "LinearColor Structure" :default (struct :`R` 1.0 :`G` 0.116667)))
  (`|SpawnActorFromClass` "/Game/Blueprint/BP_Project_Secondary.BP_Project_Secondary_C" Spawn "AlwaysSpawn" "OverrideRootScale" null (`local.Colour`) null)
  (`GameplayStatics.PlaySoundAtLocation` "/Game/Asset/Audio/PlayerShot/Shut_Down2.Shut_Down2" (`self.K2_GetActorLocation`) (struct) 1.0 1.0 0.0 null null null))

(fn `UserConstructionScript`
  (set `self.Health` (`self.MaxHealth`))
  (`SceneComponent.SetVisibility` (`self.debug coord`) (`self.show debub coord`) false))