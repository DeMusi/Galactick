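; Game mode that tracks score (named Scope), top score and enemy counts, and manages the HUD and game-over screen.
; BeginPlay sets game-only input and adds the HUD; GameOver shows its widget with cursor and UI-only input.
; LoadScope and SaveScope are empty stubs, and PlayCamSnake triggers world camera shakes.
; UpdateEnemyCount ignores its argument and always adds one, so EnemyKilled raises EnemyCount despite passing minus one.
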(event `self.ReceiveBeginPlay`
  (`WidgetBlueprintLibrary.SetInputMode_GameOnly` (`GameplayStatics.GetPlayerController` 0))
  (`self.LoadScope`)
  (`self.SetScope` 0)
  (bind _returnvalue (`|CreateWidget` "/Game/Asset/HUD/BPW_HUD.BPW_HUD_C"))
  (bind _output_get (set `self.BPW_HUD` _returnvalue))
  (`UserWidget.AddToViewport` _output_get 0))

(event `UpdateEnemyCount`
  (params (Val :type Integer))
  (`self.UpdateEnemyScope` 1))

(event `self.ReceiveEndPlay`
  (params (EndPlayReason :type "EEndPlayReason Enum" :default "Destroyed"))
  (`self.SaveScope`))

(fn `EnemyKilled`
  (`/Engine/EditorBlueprintResources/StandardMacros.IncrementInt` (`self.EnemiesKilled`)
    (:`  `
      (`self.UpdateEnemyCount` -1))))

(fn `GameOver`
  (bind _returnvalue (`GameplayStatics.GetPlayerController` 0))
  (bind _returnvalue_2 (`|CreateWidget` "/Game/Asset/HUD/BPW_GameOver.BPW_GameOver_C"))
  (`UserWidget.AddToViewport` _returnvalue_2 0)
  (set `PlayerController.bShowMouseCursor` true _returnvalue)
  (`WidgetBlueprintLibrary.SetInputMode_UIOnlyEx` _returnvalue _returnvalue_2))

(fn `LoadScope`)

(fn `PlayCamSnake`
  (params (Shake :type "CameraShake Class Reference") (Epicenter :type "Vector Structure"))
  (`GameplayStatics.PlayWorldCameraShake` Shake Epicenter 0.0 1000.0))

(fn `SaveScope`)

(fn `SetScope`
  (params (Val :type Integer))
  (bind _output_get (set `self.Scope` (+ Val (`self.Scope`))))
  (if (>= _output_get (`self.TopScope`))
    (set `self.TopScope` (`self.Scope`))
    (else
      (set `self.TopScope` (`self.TopScope`)))))

(fn `UpdateEnemyScope`
  (params (Val :type Integer))
  (set `self.EnemyCount` (+ (`self.EnemyCount`) Val)))

(fn `UserConstructionScript`)