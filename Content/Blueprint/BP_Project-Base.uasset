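; Base projectile actor that damages whatever its mesh overlaps, spawns a pixel explosion emitter at its location and destroys itself.
; The construction script creates a dynamic material on the mesh and applies the Scale and Speed variables to the mesh and projectile movement.
; BeginPlay tints that material with ProjectColour, so size, speed, colour and damage are all driven by variables.
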(event `self.ReceiveBeginPlay`
  (`MaterialInstanceDynamic.SetVectorParameterValue` (`self.ProjectMat`) "Colour" (`self.ProjectColour`)))

(event `self.StaticMesh.OnComponentBeginOverlap`
  (params (OverlappedComponent :type "PrimitiveComponent Object Reference") (OtherActor :type "Actor Object Reference") (OtherComp :type "PrimitiveComponent Object Reference") (OtherBodyIndex :type Integer) (bFromSweep :type Boolean) (SweepResult :type "HitResult Structure (by ref)"))
  (`GameplayStatics.ApplyDamage` OtherActor (`self.Damage`))
  (`GameplayStatics.SpawnEmitterAtLocation` "/Game/Asset/Particles/P_Pixel_Explosion.P_Pixel_Explosion" (`self.K2_GetActorLocation`))
  (`self.K2_DestroyActor`))

(fn `UserConstructionScript`
  (bind _projectilemovement (`self.ProjectileMovement`))
  (bind _returnvalue (`PrimitiveComponent.CreateDynamicMaterialInstance` (`self.StaticMesh`) 0 null "None"))
  (set `self.ProjectMat` _returnvalue)
  (`SceneComponent.SetWorldScale3D` (`self.StaticMesh`) (`self.Scale`))
  (bind _output_get (set `ProjectileMovementComponent.MaxSpeed` (`self.Speed`) _projectilemovement))
  (set `ProjectileMovementComponent.InitialSpeed` _output_get _projectilemovement))