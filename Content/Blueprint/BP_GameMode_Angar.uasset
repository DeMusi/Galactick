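; BP_GameMode_Angar is a game mode that opens the BPW_Start widget on BeginPlay, after clearing all other widgets and showing the mouse cursor.
; It also provides save helpers that BeginPlay does not call.
; LoadData returns a named slot as SaveOptions, or nothing if the slot is missing or the cast fails.
; SaveData writes to a named slot, replacing an existing save only when Overwrite is set.
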(event `self.ReceiveBeginPlay`
  (`WidgetLayoutLibrary.RemoveAllWidgets`)
  (bind _returnvalue (`|CreateWidget` "/Game/Asset/HUD/BPW_Start.BPW_Start_C"))
  (`UserWidget.AddToViewport` _returnvalue 0)
  (set `PlayerController.bShowMouseCursor` true (`GameplayStatics.GetPlayerController` 0)))

(fn `LoadData`
  (params (FileNAme :type String))
  (returns (Data :type "/Game/Blueprint/SaveGame/SaveOptions Object Reference"))
  (`GameplayStatics.DoesSaveGameExist` FileNAme)
  (if true
    (bind _returnvalue (`GameplayStatics.LoadGameFromSlot` FileNAme))
    (bind _assave_options (cast `/Game/Blueprint/SaveGame/SaveOptions` _returnvalue)
      (:`then`
        (return _assave_options))
      (:`CastFailed`
        _)))
  (return null))

(fn `SaveData`
  (params (Data2 :type "/Game/Blueprint/SaveGame/SaveOptions Object Reference") (FileName :type String) (Overwrite :type Boolean))
  (bind _returnvalue (`GameplayStatics.DoesSaveGameExist` FileName))
  (if _returnvalue
    (if Overwrite
      (`GameplayStatics.SaveGameToSlot` Data2 FileName :!label _label))
    (else
      (goto _label))))

(fn `UserConstructionScript`)